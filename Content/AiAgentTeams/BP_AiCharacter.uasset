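; AI character Blueprint that turns to face actors it sees through its AI Perception component.
; Each Tick, it takes the last actor in the currently perceived sight list and snaps its yaw toward that actor's location.
; Team logic is unfinished: AssignTeam only returns false, and an attitude check in the construction script is never executed.
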(event `self.ReceiveBeginPlay`)

(event `self.ReceiveTick`
  (params (DeltaSeconds :type "Float (single-precision)"))
  (bind _outactors (`AIPerceptionComponent.GetCurrentlyPerceivedActors` (`self.AIPerception`) "/Script/AIModule.AISense_Sight"))
  (bind _returnvalue (`KismetArrayLibrary.Array_Length` _outactors))
  (bind (_returnvalue_roll _returnvalue_pitch _returnvalue_yaw) (`KismetMathLibrary.BreakRotator` (`KismetMathLibrary.FindLookAtRotation` (`self.K2_GetActorLocation`) (`self.K2_GetActorLocation` (`|GetArrayItem` _outactors (- _returnvalue 1))))))
  (if (> _returnvalue 0)
    (`self.K2_SetActorRotation` (`KismetMathLibrary.MakeRotator` 0.0 0.0 _returnvalue_yaw))))

(fn `AssignTeam`
  (params (InTeam :type "AgentTeam Object Reference"))
  (returns (ReturnValue :type Boolean))
  (return false))

(fn `UserConstructionScript`)